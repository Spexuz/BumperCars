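; Drivable car pawn with hand-built raycast-style vehicle physics on a single physics body.
; Each async physics tick, four sphere-traced suspension points apply spring-damper forces, while tire forces counter sideways slip.
; Move input applies engine force at all wheels, angling the front pair for steering and adding yaw torque when driving forward.
; Tick separately re-traces to animate wheel height, smoothed steering, clamped camber and speed-based spin.
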(event `self.ReceiveTick`
  (params (DeltaSeconds :type "Float (single-precision)"))
  (bind _m_pphysicsbody (`self.m_pPhysicsBody`))
  (`|ExecutionSequence`
    (:`then_0`
      (`self.UpdateVisual` (`self.S_BR_SuspensionPoint`) (`self.SM_BR_Wheel`))
      (`self.UpdateVisual` (`self.S_FL_SuspensionPoint`) (`self.SM_FL_Wheel`) true)
      (`self.UpdateVisual` (`self.S_FR_SuspensionPoint`) (`self.SM_FR_Wheel`) true)
      (`self.UpdateVisual` (`self.S_BL_SuspensionPoint`) (`self.SM_BL_Wheel`)))
    (:`then_1`
      (bind _returnvalue (`PrimitiveComponent.GetPhysicsLinearVelocity` _m_pphysicsbody "None"))
      (set `self.m_fAcceleration` (`KismetMathLibrary.Dot_VectorVector` _returnvalue (`SceneComponent.GetForwardVector` _m_pphysicsbody))))))

(event `self.ReceiveAsyncPhysicsTick`
  (params (DeltaSeconds :type "Float (single-precision)") (SimSeconds :type "Float (single-precision)"))
  (bind _s_br_suspensionpoint (`self.S_BR_SuspensionPoint`))
  (bind _s_fl_suspensionpoint (`self.S_FL_SuspensionPoint`))
  (bind _s_fr_suspensionpoint (`self.S_FR_SuspensionPoint`))
  (bind _s_bl_suspensionpoint (`self.S_BL_SuspensionPoint`))
  (`self.SimulateSuspensionSpring` _s_br_suspensionpoint)
  (`self.SimulateTire` _s_br_suspensionpoint (`self.SM_BR_Wheel`))
  (`self.SimulateSuspensionSpring` _s_fl_suspensionpoint)
  (`self.SimulateTire` _s_fl_suspensionpoint (`self.SM_FL_Wheel`))
  (`self.SimulateSuspensionSpring` _s_fr_suspensionpoint)
  (`self.SimulateTire` _s_fr_suspensionpoint (`self.SM_FR_Wheel`))
  (`self.SimulateSuspensionSpring` _s_bl_suspensionpoint)
  (`self.SimulateTire` _s_bl_suspensionpoint (`self.SM_BL_Wheel`)))

(event `EnhancedInput|/Game/Data/Input/IA/IA_Move`
  (params (ActionValue :type "Vector2D Structure") (ElapsedSeconds :type "Float (double-precision)") (TriggeredSeconds :type "Float (double-precision)") (InputAction :type "InputAction Object Reference" :default "/Game/Data/Input/IA/IA_Move.IA_Move"))
  (:`Triggered`
    (`|ExecutionSequence`
      (:`then_0`
        (`self.ControlBackWheel` (`self.SM_BR_Wheel`))
        (`self.ControlBackWheel` (`self.SM_BL_Wheel`)))
      (:`then_1`
        (`self.ControlFrontWheel` (`self.SM_FL_Wheel`))
        (`self.ControlFrontWheel` (`self.SM_FR_Wheel`)))))
  (:`Completed`
    (set `self.m_fTargetSteeringAngle` 0.0)))

(fn `Calculate Spring Force`
  (params (Distance :type "Float (double-precision)"))
  (returns (`Spring Force` :type "Float (double-precision)"))
  (return (* (`KismetMathLibrary.FMax` (- (`self.m_fSpringRestLength`) (`KismetMathLibrary.FClamp` Distance (`self.m_fMinSpringRange`) (`self.m_fMaxSpringRange`)))) (`self.m_fSpringStiffness`))))

(fn `Calulate Dampening Force`
  (params (Distance :type "Float (double-precision) (by ref)") (`Previous Distance` :type "Float (double-precision) (by ref)"))
  (returns (`Dampening Force` :type "Float (double-precision)"))
  (return (* (/ (- `Previous Distance` Distance) (`GameplayStatics.GetWorldDeltaSeconds`)) (`self.m_fSpringDampening`))))

(fn `ControlBackWheel`
  (params (`Wheel Ref` :type "StaticMeshComponent Object Reference (by ref)"))
  (`PrimitiveComponent.AddForceAtLocation` (`self.m_pPhysicsBody`) (* (`SceneComponent.GetForwardVector` (`self.m_pPhysicsBody`)) (* (`self.m_fInput_YAxis`) (`self.m_fEngineForce`))) (`SceneComponent.K2_GetComponentLocation` (`local.Wheel Ref`)) "None"))

(fn `ControlFrontWheel`
  (params (`Wheel Ref` :type "StaticMeshComponent Object Reference (by ref)"))
  (bind _m_pphysicsbody (`self.m_pPhysicsBody`))
  (bind _returnvalue (* (`self.m_fMaxTurnAngle`) (`self.m_fInput_XAxis`)))
  (set `self.m_fTargetSteeringAngle` _returnvalue)
  (`PrimitiveComponent.AddForceAtLocation` (`self.m_pPhysicsBody`) (* (`self.m_fInput_YAxis`) (`self.m_fEngineForce`) (`KismetMathLibrary.RotateAngleAxis` (`SceneComponent.GetForwardVector` _m_pphysicsbody) _returnvalue (`SceneComponent.GetUpVector` _m_pphysicsbody))) (`SceneComponent.K2_GetComponentLocation` (`local.Wheel Ref`)) "None")
  (if (> (`self.m_fInput_YAxis`) 0.0)
    (`PrimitiveComponent.AddTorqueInRadians` (`self.m_pPhysicsBody`) (`KismetMathLibrary.MakeVector` 0.0 0.0 (* (`self.m_fTargetSteeringAngle`) (`self.m_fEngineTorque`))) "None" false)))

(fn `SimulateSuspensionSpring`
  (params (`Suspension Point Ref` :type "SceneComponent Object Reference (by ref)"))
  (locals (fSpringMaxLength :type "Float (double-precision)" :default 0.0) (`Spring Force` :type "Float (double-precision)" :default 0.0))
  (bind _returnvalue (`SceneComponent.K2_GetComponentLocation` `Suspension Point Ref`))
  ; Set up Spring Details
  ; Sphere Trace to Simulate Volume
  (bind (_outhit _returnvalue_2) (`KismetSystemLibrary.SphereTraceSingle` :`Start` _returnvalue :`End` (+ _returnvalue (* (* (`SceneComponent.GetUpVector` (`self.m_pPhysicsBody`)) (+ (`self.m_fSpringRestLength`) (`self.m_fSpringTravel`))) -1.0)) :`Radius` (`self.m_fWheelRadius`) :`TraceChannel` "TraceTypeQuery1" :`DrawDebugType` "ForOneFrame"))
  (if _returnvalue_2
    ; Fetch True Velocity from Spring
    (bind _returnvalue_3 (`PrimitiveComponent.GetPhysicsLinearVelocityAtPoint` (`self.m_pPhysicsBody`) (`SceneComponent.K2_GetComponentLocation` (`local.Suspension Point Ref`)) "None"))
    (bind (_bblockinghit _binitialoverlap _time _distance _location _impactpoint _normal _impactnormal) (`GameplayStatics.BreakHitResult` _outhit))
    ; Apply Final Vector Force to Spring
    (`PrimitiveComponent.AddForceAtLocation` (`self.m_pPhysicsBody`) (* (+ (* (* (`KismetMathLibrary.Dot_VectorVector` _returnvalue_3 _impactnormal) -1.0) (`self.m_fSpringDampening`)) (`self.Calculate Spring Force` _distance)) _impactnormal) (`SceneComponent.K2_GetComponentLocation` (`local.Suspension Point Ref`)) "None")))

(fn `SimulateTire`
  (params (`Suspension Ref` :type "SceneComponent Object Reference") (`Wheel Ref` :type "StaticMeshComponent Object Reference"))
  (bind _returnvalue (`PrimitiveComponent.GetPhysicsLinearVelocityAtPoint` (`self.m_pPhysicsBody`) (`SceneComponent.K2_GetComponentLocation` `Suspension Ref`) "None"))
  (`PrimitiveComponent.AddForceAtLocation` (`self.m_pPhysicsBody`) (* (* (* (`KismetMathLibrary.Dot_VectorVector` _returnvalue (`SceneComponent.GetRightVector` `Wheel Ref`)) 10000.0) -1.0) (`SceneComponent.GetRightVector` (`local.Wheel Ref`))) (`SceneComponent.K2_GetComponentLocation` (`local.Suspension Ref`)) "None"))

(fn `UpdateVisual`
  (params (`Suspension Ref` :type "SceneComponent Object Reference") (`Wheel Ref` :type "StaticMeshComponent Object Reference") (`Should Steer` :type Boolean))
  (bind _returnvalue (`SceneComponent.K2_GetComponentLocation` `Suspension Ref`))
  (bind _wheel_ref (`local.Wheel Ref`))
  (bind _returnvalue_2 (* (`self.m_fAcceleration`) 1.2))
  (bind _relativerotation_roll (`KismetMathLibrary.BreakRotator` (`SceneComponent.RelativeRotation` (`self.m_pPhysicsBody`))))
  (bind _returnvalue_3 (* (`KismetMathLibrary.FClamp` _relativerotation_roll (`self.m_fMinCamber`) (`self.m_fMaxCamber`)) -1.0))
  ; Sphere Trace for Volumetric Updates
  (bind (_outhit _returnvalue_4) (`KismetSystemLibrary.SphereTraceSingle` :`Start` _returnvalue :`End` (+ _returnvalue (* (* (`SceneComponent.GetUpVector` (`self.m_pPhysicsBody`)) (+ (`self.m_fSpringRestLength`) (`self.m_fSpringTravel`))) -1.0)) :`Radius` (`self.m_fWheelRadius`) :`TraceChannel` "TraceTypeQuery1" :`DrawDebugType` "ForOneFrame" :`TraceColor` (struct :`R` 0.954094 :`G` 0.956389 :`B` 1.0 :`A` 1.0) :`TraceHitColor` (struct :`R` 0.470239 :`G` 0.463218 :`B` 1.0 :`A` 1.0)))
  (if _returnvalue_4
    ; Visualize Spring Compression
    (`SceneComponent.K2_SetRelativeLocation` (`local.Wheel Ref`) (`KismetMathLibrary.MakeVector` 0.0 0.0 (* (`KismetMathLibrary.FClamp` (`.Distance` (`GameplayStatics.BreakHitResult` _outhit)) (`self.m_fMinSpringRange`) (`self.m_fMaxSpringRange`)) -1.0)) false false)
    (if (`local.Should Steer`)
      ; Update Rolling/Turning for All & Front Wheels respectivly
      (bind _output_get (set `self.m_fCurrentSteeringAngle` (`KismetMathLibrary.FInterpTo` (`self.m_fCurrentSteeringAngle`) (`self.m_fTargetSteeringAngle`) (`GameplayStatics.GetWorldDeltaSeconds`) 1.0)))
      (`SceneComponent.K2_SetRelativeRotation` _wheel_ref (`KismetMathLibrary.MakeRotator` _returnvalue_3 0.0 _output_get) false false)
      (`SceneComponent.K2_AddRelativeRotation` _wheel_ref (`KismetMathLibrary.MakeRotator` 0.0 _returnvalue_2) false false)
      (else
        (`SceneComponent.K2_SetRelativeRotation` (`local.Wheel Ref`) (`KismetMathLibrary.MakeRotator` _returnvalue_3 0.0 0.0) false false)
        (`SceneComponent.K2_AddRelativeRotation` (`local.Wheel Ref`) (`KismetMathLibrary.MakeRotator` 0.0 _returnvalue_2) false false)))))

(fn `UserConstructionScript`)
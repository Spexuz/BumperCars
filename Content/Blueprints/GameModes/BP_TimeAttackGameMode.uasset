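; Game mode for a time attack racing game that handles the main menu and spawning the player's car.
; On BeginPlay it points the view at the camera tagged for the main menu and shows the menu widget with UI-only input and a visible cursor.
; The IStartRace interface event spawns BP_Car at the player start and has the first player controller possess it.
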(event `self.ReceiveBeginPlay`
  (`self.Setup Main Menu`))

(event `/Game/Blueprints/GameModes/GMInterfaces/BPI_GameMode.IStartRace`
  (`self.Start Race`))

(fn `Setup Main Menu`
  (bind _returnvalue (`GameplayStatics.GetPlayerController` 0))
  ; Setup Main Menu
  (bind _outactors (`GameplayStatics.GetAllActorsOfClassWithTag` "/Script/Engine.CameraActor" "C_MainMenu"))
  (`PlayerController.SetViewTargetWithBlend` (`GameplayStatics.GetPlayerController` 0) (`|GetArrayItem` _outactors) 0.0 "VTBlend_Linear" 0.0 false)
  (bind _returnvalue_2 (`|CreateWidget` "/Game/Blueprints/Widgets/WBP_MainMenu.WBP_MainMenu_C" _returnvalue))
  (`UserWidget.AddToViewport` _returnvalue_2 0)
  (`WidgetBlueprintLibrary.SetInputMode_UIOnlyEx` _returnvalue _returnvalue_2 "DoNotLock" true)
  (set `PlayerController.bShowMouseCursor` true (`GameplayStatics.GetPlayerController` 0)))

(fn `Start Race`
  (bind _returnvalue (`|SpawnActorFromClass` "/Game/Blueprints/Pawns/BP_Car.BP_Car_C" (`self.GetTransform` (`self.K2_FindPlayerStart` (`GameplayStatics.GetPlayerController` 0))) "Undefined" "MultiplyWithRoot" (`Controller.K2_GetPawn` (`GameplayStatics.GetPlayerController` 0)) null))
  (`Controller.Possess` (`GameplayStatics.GetPlayerController` 0) _returnvalue))

(fn `UserConstructionScript`)